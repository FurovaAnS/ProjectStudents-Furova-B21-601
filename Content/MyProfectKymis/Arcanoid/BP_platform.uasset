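; BP_platform is the player-controlled paddle in an Arkanoid game.
; The MoveRight input axis slides it left or right along local Y in fixed sweeping steps, ignoring the axis magnitude.
; When a BP_bonus overlaps its Cube, it destroys the bonus and calls TwoBalls, which spawns an extra BP_ball at the Arrow component's location.
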(event `InputAxis|MoveRight`
  (params (AxisValue :type "Float (single-precision)"))
  (if (> AxisValue 0.0)
    (`self.K2_AddActorLocalOffset` (0.0 25.0 0.0) true)))

(event `InputAxis|MoveRight`
  (params (AxisValue :type "Float (single-precision)"))
  (if (< AxisValue 0.0)
    (`self.K2_AddActorLocalOffset` (0.0 -25.0 0.0) true)))

(event `self.Cube.OnComponentBeginOverlap`
  (params (OverlappedComponent :type "PrimitiveComponent Object Reference") (OtherActor :type "Actor Object Reference") (OtherComp :type "PrimitiveComponent Object Reference") (OtherBodyIndex :type Integer) (bFromSweep :type Boolean) (SweepResult :type "HitResult Structure (by ref)"))
  (bind _asbp_bonus (cast `/Game/MyProfectKymis/Arcanoid/BP_bonus` OtherActor))
  (`self.K2_DestroyActor` _asbp_bonus)
  (`self.TwoBalls`))

(event `TwoBalls`
  (`|SpawnActorFromClass` "/Game/MyProfectKymis/Arcanoid/BP_ball.BP_ball_C" (`KismetMathLibrary.MakeTransform` (`SceneComponent.K2_GetComponentLocation` (`self.Arrow`))) "AlwaysSpawn" "OverrideRootScale" null null))

(fn `UserConstructionScript`)